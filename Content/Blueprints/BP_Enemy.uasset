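; BP_Enemy is an enemy actor that travels along the spline of a randomly chosen Connector actor, picked at BeginPlay.
; MoveCharacter scales the EnemyMover timeline's play rate by Duration, sets its start time from CartOffset, then plays it.
; Each update converts the timeline's Alpha into a distance along the spline, sets world location and rotation there, and prints the location to screen.
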(event `self.ReceiveBeginPlay`
  (bind _outactors (`GameplayStatics.GetAllActorsOfClass` "/Script/GridRunner_PoC.Connector"))
  (bind _returnvalue (`Connector.GetSpline` (`KismetArrayLibrary.Array_Random` _outactors)))
  (set `self.EnemyConnector` _returnvalue)
  (`self.MoveCharacter`))

(event `MoveCharacter`
  (bind _enemymover (`self.EnemyMover`))
  (bind _enemyconnector (`self.EnemyConnector`))
  (bind _returnvalue (`KismetMathLibrary.Lerp` 0.0 (`SplineComponent.GetSplineLength` _enemyconnector) (`self.Alpha`)))
  (bind _returnvalue_2 (`SplineComponent.GetLocationAtDistanceAlongSpline` _enemyconnector _returnvalue "World"))
  (`TimelineComponent.SetPlayRate` _enemymover (/ 1.0 (`self.Duration`)))
  (`TimelineComponent.SetNewTime` _enemymover (`self.CartOffset`))
  (bind (_direction _alpha) (`Timeline|EnemyMover`)
    (:`Update`
      (set `self.Alpha` _alpha)
      (`self.K2_SetActorLocationAndRotation` _returnvalue_2 (`SplineComponent.GetRotationAtDistanceAlongSpline` _enemyconnector _returnvalue "World"))
      (`KismetSystemLibrary.PrintString` (`KismetStringLibrary.Conv_VectorToString` _returnvalue_2)))))

(fn `UserConstructionScript`)
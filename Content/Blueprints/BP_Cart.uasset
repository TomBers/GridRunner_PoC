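; BP_Cart is an actor that rides along a spline track when active at BeginPlay.
; MoveCart scales the CartMover timeline's play rate by the inverse of Duration and seeks it to CartOffset before playing.
; Each timeline update maps Alpha to a distance along TrackRef's root spline and sets the cart's world location and rotation from that point.
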(event `self.ReceiveBeginPlay`
  (if (`self.IsActive`)
    (`self.MoveCart`)))

(event `MoveCart`
  (bind _cartmover (`self.CartMover`))
  (`TimelineComponent.SetPlayRate` _cartmover (/ 1.0 (`self.Duration`)))
  (`TimelineComponent.SetNewTime` _cartmover (`self.CartOffset`))
  (bind _asspline_component (cast `SplineComponent` (`Actor.RootComponent` (`self.TrackRef`))))
  (bind (_direction _alpha) (`Timeline|CartMover`)
    (:`Update`
      (set `self.Alpha` _alpha)
      (bind _returnvalue (`KismetMathLibrary.Lerp` 0.0 (`SplineComponent.GetSplineLength` _asspline_component) (`self.Alpha`)))
      (`self.K2_SetActorLocationAndRotation` (`SplineComponent.GetLocationAtDistanceAlongSpline` _asspline_component _returnvalue "World") (`SplineComponent.GetRotationAtDistanceAlongSpline` _asspline_component _returnvalue "World")))))

(fn `UserConstructionScript`)
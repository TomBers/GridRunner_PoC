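; BP_Point is a point marker actor whose Sphere reflects state set through actor tags.
; Every Tick, it hides the Sphere if the actor is tagged HIDDEN and colours it red if tagged GRABBED, otherwise blue.
; The colour is applied by creating a new dynamic instance of PointMaterial each frame and setting its PointColour parameter, with no caching of the instance.
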(event `self.ReceiveBeginPlay`)

(event `self.ReceiveTick`
  (params (DeltaSeconds :type "Float (single-precision)"))
  (bind _sphere (`self.Sphere`))
  (`SceneComponent.SetVisibility` (`self.Sphere`) (not (`self.ActorHasTag` "HIDDEN")) false)
  (if (`self.ActorHasTag` "GRABBED")
    (bind _returnvalue (`PrimitiveComponent.CreateDynamicMaterialInstance` _sphere 0 "/Game/PointMaterial.PointMaterial" "None"))
    (`MaterialInstanceDynamic.SetVectorParameterValue` _returnvalue "PointColour" (struct :`R` 0.530741 :`G` 0.06654 :`B` 0.073758 :`A` 1.0))
    (else
      (bind _returnvalue_2 (`PrimitiveComponent.CreateDynamicMaterialInstance` _sphere 0 "/Game/PointMaterial.PointMaterial" "None"))
      (`MaterialInstanceDynamic.SetVectorParameterValue` _returnvalue_2 "PointColour" (struct :`R` 0.027749 :`G` 0.074922 :`B` 0.529053 :`A` 1.0)))))

(fn `UserConstructionScript`)
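; Character Blueprint that rides along a Connector's spline like a cart, matching the spline's location and rotation.
; BeginPlay starts the ride on the existing spline reference when IsActive, otherwise it sets movement to Flying.
; StartButton picks a random Connector's spline and starts the ride.
; The CartMover timeline drives distance along the spline, with play rate derived from Duration and start time from CartOffset.
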(event `InputAction|StartButton`
  (params (Key :type "Key Structure"))
  (:`Pressed`
    (bind _outactors (`GameplayStatics.GetAllActorsOfClass` "/Script/GridRunner_PoC.Connector"))
    (bind _returnvalue (`Connector.GetSpline` (`KismetArrayLibrary.Array_Random` _outactors)))
    (set `self.ConnectorSplineRef` _returnvalue)
    (`self.MoveCharacter`)))

(event `self.ReceiveBeginPlay`
  (if (`self.IsActive`)
    (`self.MoveCharacter`)
    (else
      (`CharacterMovementComponent.SetMovementMode` (`self.CharacterMovement`) "MOVE_Flying" 0))))

(event `MoveCharacter`
  (bind _connectorsplineref (`self.ConnectorSplineRef`))
  (bind _cartmover (`self.CartMover`))
  (bind _returnvalue (`KismetMathLibrary.Lerp` 0.0 (`SplineComponent.GetSplineLength` _connectorsplineref) (`self.Alpha`)))
  (`TimelineComponent.SetPlayRate` _cartmover (/ 1.0 (`self.Duration`)))
  (`TimelineComponent.SetNewTime` _cartmover (`self.CartOffset`))
  (bind (_direction _alpha) (`Timeline|CartMover`)
    (:`Update`
      (set `self.Alpha` _alpha)
      (`self.K2_SetActorLocationAndRotation` (`SplineComponent.GetLocationAtDistanceAlongSpline` _connectorsplineref _returnvalue "World") (`SplineComponent.GetRotationAtDistanceAlongSpline` _connectorsplineref _returnvalue "World")))))

(fn `UserConstructionScript`)